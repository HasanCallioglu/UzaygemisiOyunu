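; BP_MainCharacter is the player character Blueprint, providing basic movement, camera look and HUD setup.
; BeginPlay creates a WB_HUD widget for player 0, stores it and adds it to the viewport.
; Turkish-named axis inputs drive forward/back and strafe movement relative to control yaw only, ignoring pitch and roll.
; The look axes feed controller rotation directly, with bakma_x driving pitch and bakma_y driving yaw.
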(event EventBeginPlay
  (bind _returnvalue (UserInterface|CreateWidget "/Game/IU/WB_HUD.WB_HUD_C" (Game|GetPlayerController 0)))
  (bind _output_get (Variables|Default|SetHUD%20Widget _returnvalue))
  (UserInterface|Viewport|AddtoViewport _output_get 0))

(event Input|AxisEvents|InputAxisileri-geri
  (params (AxisValue :type Float%20%28single-precision%29))
  ;[1 1 1] movment
  (Pawn|Input|AddMovementInput (Math|Vector|GetForwardVector (Math|Rotator|MakeRotator 0.0 0.0 (.Yaw (Math|Rotator|BreakRotator (Pawn|GetControlRotation :!class /Script/Engine.Pawn))))) AxisValue false))

(event Input|AxisEvents|InputAxissağ-sol
  (params (AxisValue :type Float%20%28single-precision%29))
  ;[1 1 1] movment
  (Pawn|Input|AddMovementInput (Math|Vector|GetRightVector (Math|Rotator|MakeRotator 0.0 0.0 (.Yaw (Math|Rotator|BreakRotator (Pawn|GetControlRotation :!class /Script/Engine.Pawn))))) AxisValue false))

(event Input|AxisEvents|InputAxisbakma_x
  (params (AxisValue :type Float%20%28single-precision%29))
  ;[1 1 1] movment
  (Pawn|Input|AddControllerPitchInput AxisValue))

(event Input|AxisEvents|InputAxisbakma_y
  (params (AxisValue :type Float%20%28single-precision%29))
  ;[1 1 1] movment
  (Pawn|Input|AddControllerYawInput AxisValue))

(fn ConstructionScript)