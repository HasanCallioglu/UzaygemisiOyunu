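; Player stats component for BP_MainCharacter, largely an unfinished stub.
; BeginPlay caches its owner as the main character.
; GetMoney does nothing, as its logic to print BP_BASE's MeteorMoney and show it on the HUD is disconnected.
; SafeZone only casts the player pawn to BP_BASE and stores it, leaving InSafeZone unused.
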(event EventBeginPlay
  (bind _asbp_main_character (Utilities|Casting|CastToBP_MainCharacter (Components|GetOwner)))
  (Variables|Default|SetAs%20BP%20Main%20Character _asbp_main_character)
  (if true
    _))

(event EventTick
  (params (DeltaSeconds :type Float%20%28single-precision%29)))

(fn GetMoney)

(fn SafeZone
  (bind _asbp_base (Utilities|Casting|CastToBP_BASE (Game|Player|GetPlayerPawn 0)))
  (bind _output_get (Variables|Default|SetAs%20BP%20BASE_0 _asbp_base)))