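; BP_Base1 is a base actor that pays the player for meteors brought into it and tracks whether the player is in its safe zone.
; When a BP_Meteor overlaps Box, it adds 100 to its own MeteorMoney total and overwrites the main character's Money with that total.
; Triger flips InSafeZone whenever a Player-tagged actor begins or ends overlap, rather than setting it explicitly.
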(event OnComponentBeginOverlap(Box)
  (params (OverlappedComponent :type Primitive%20Component%20Object%20Reference) (OtherActor :type Actor%20Object%20Reference) (OtherComp :type Primitive%20Component%20Object%20Reference) (OtherBodyIndex :type Integer) (bFromSweep :type Boolean) (SweepResult :type Hit%20Result%20Structure%20%28by%20ref%29))
  (Utilities|Casting|CastToBP_Meteor OtherActor)
  (bind _asbp_main_character (Utilities|Casting|CastToBP_MainCharacter (Game|GetPlayerCharacter 0)))
  (Variables|Default|SetAs%20BP%20Main%20Character _asbp_main_character)
  (bind _output_get (Variables|Default|SetMeteor%20Money (+ (Variables|Default|GetMeteor%20Money) 1e+02)))
  (bind _output_get_2 (Variables|/Game/MainCharakter/BP_MainCharacter.BP_MainCharacter_C|SetMoney (Variables|Default|GetAs%20BP%20Main%20Character) _output_get))
  (Development|PrintString (Utilities|String|ToString(Float) _output_get_2)))

(event OnComponentHit(Cube)
  (params (HitComponent :type Primitive%20Component%20Object%20Reference) (OtherActor :type Actor%20Object%20Reference) (OtherComp :type Primitive%20Component%20Object%20Reference) (NormalImpulse :type Vector :default "0, 0, 0") (Hit :type Hit%20Result%20Structure%20%28by%20ref%29)))

(event OnComponentBeginOverlap(Triger)
  (params (OverlappedComponent :type Primitive%20Component%20Object%20Reference) (OtherActor :type Actor%20Object%20Reference) (OtherComp :type Primitive%20Component%20Object%20Reference) (OtherBodyIndex :type Integer) (bFromSweep :type Boolean) (SweepResult :type Hit%20Result%20Structure%20%28by%20ref%29))
  (if (Actor|ActorHasTag OtherActor "Player")
    (Development|PrintString "start")
    (bind _output_get (Variables|Default|SetIn%20Safe%20Zone (not (Variables|Default|GetIn%20Safe%20Zone))))
    (if _output_get
      (Variables|Default|SetIn%20Safe%20Zone true)
      (else
        (Variables|Default|SetIn%20Safe%20Zone false)))))

(event OnComponentEndOverlap(Triger)
  (params (OverlappedComponent :type Primitive%20Component%20Object%20Reference) (OtherActor :type Actor%20Object%20Reference) (OtherComp :type Primitive%20Component%20Object%20Reference) (OtherBodyIndex :type Integer))
  (if (Actor|ActorHasTag OtherActor "Player")
    (Development|PrintString "start")
    (bind _output_get (Variables|Default|SetIn%20Safe%20Zone (not (Variables|Default|GetIn%20Safe%20Zone))))
    (if _output_get
      (Variables|Default|SetIn%20Safe%20Zone true)
      (else
        (Variables|Default|SetIn%20Safe%20Zone false)))))

(event EventBeginPlay)

(event Collision|EventActorBeginOverlap
  (params (OtherActor :type Actor%20Object%20Reference)))

(event EventTick
  (params (DeltaSeconds :type Float%20%28single-precision%29)))

(fn ConstructionScript)