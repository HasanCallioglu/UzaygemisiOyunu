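; Base actor that credits the player with money when a BP_Meteor enters its Box volume.
; Each overlap adds a fixed amount to a running MeteorMoney total, overwrites the first player's BP_MainCharacter Money with that total, and prints it.
; A separate Triger volume only prints debug text when a Player-tagged actor enters or leaves.
; A BP_Meteor_2 cast is present but never runs.
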(event OnComponentBeginOverlap(Box)
  (params (OverlappedComponent :type Primitive%20Component%20Object%20Reference) (OtherActor :type Actor%20Object%20Reference) (OtherComp :type Primitive%20Component%20Object%20Reference) (OtherBodyIndex :type Integer) (bFromSweep :type Boolean) (SweepResult :type Hit%20Result%20Structure%20%28by%20ref%29))
  (Utilities|Casting|CastToBP_Meteor OtherActor)
  (bind _asbp_main_character (Utilities|Casting|CastToBP_MainCharacter (Game|GetPlayerCharacter 0)))
  (Variables|Default|SetAs%20BP%20Main%20Character _asbp_main_character)
  (bind _output_get (Variables|Default|SetMeteorMoney (+ (Variables|Default|GetMeteorMoney) 1e+02)))
  (bind _output_get_2 (Variables|/Game/MainCharakter/BP_MainCharacter.BP_MainCharacter_C|SetMoney (Variables|Default|GetAs%20BP%20Main%20Character) _output_get))
  (Development|PrintString (Utilities|String|ToString(Float) _output_get_2)))

(event OnComponentBeginOverlap(Triger)
  (params (OverlappedComponent :type Primitive%20Component%20Object%20Reference) (OtherActor :type Actor%20Object%20Reference) (OtherComp :type Primitive%20Component%20Object%20Reference) (OtherBodyIndex :type Integer) (bFromSweep :type Boolean) (SweepResult :type Hit%20Result%20Structure%20%28by%20ref%29))
  (if (Actor|ActorHasTag OtherActor "Player")
    (Development|PrintString "Begen")
    (if true
      _)))

(event OnComponentEndOverlap(Triger)
  (params (OverlappedComponent :type Primitive%20Component%20Object%20Reference) (OtherActor :type Actor%20Object%20Reference) (OtherComp :type Primitive%20Component%20Object%20Reference) (OtherBodyIndex :type Integer))
  (if (Actor|ActorHasTag OtherActor "Player")
    (Development|PrintString "end")
    (if true
      _)))

(event EventBeginPlay)

(event Collision|EventActorBeginOverlap
  (params (OtherActor :type Actor%20Object%20Reference)))

(event EventTick
  (params (DeltaSeconds :type Float%20%28single-precision%29)))

(fn ConstructionScript)